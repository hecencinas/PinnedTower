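; BP_Bonus is a shootable bonus that advances in enemy action steps.
; A normal projectile overlapping its box destroys it and notifies the owning tower of one fixed bonus type.
; Its Act override skips the parent logic: it steps backward along its forward axis, flags overlap with BP_LastLine and notifies the game state.
; Once flagged, its next action destroys it without notifying a player hit or action completion.
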(event `self.Box.OnComponentBeginOverlap`
  (params (OverlappedComponent :type "PrimitiveComponent Object Reference") (OtherActor :type "Actor Object Reference") (OtherComp :type "PrimitiveComponent Object Reference") (OtherBodyIndex :type Integer) (bFromSweep :type Boolean) (SweepResult :type "HitResult Structure (by ref)"))
  (bind _asbp_normal_projectile (cast `/Game/Blueprints/BP_NormalProjectile` OtherActor))
  (bind _asbp_tower (cast `/Game/Blueprints/BP_Tower` (`self.GetOwner` _asbp_normal_projectile))
    (:`then`
      (`/Game/Blueprints/BP_Tower.NotifyBonus` _asbp_tower "NewEnumerator0"))
    (:`CastFailed`
      _))
  (`self.K2_DestroyActor`))

(fn `Act`
  (`/Engine/EditorBlueprintResources/StandardMacros.IncrementInt` (`self.ActionsTaken`)
    (:`  `
      (if (`self.OnLastLine`)
        (`self.K2_DestroyActor`)
        (else
          (`self.K2_AddActorWorldOffset` (* (`self.GetActorForwardVector`) -100.0))
          (if (> (`KismetArrayLibrary.Array_Length` (`PrimitiveComponent.GetOverlappingActors` (`self.Box`) "/Game/Blueprints/BP_LastLine.BP_LastLine_C")) 0)
            (set `self.OnLastLine` true))
          (`/Game/Blueprints/GameMode/BP_GameStateBase.NotifyEnemiesActionFinished` (`self.GameStateRef`)))))))

(fn `UserConstructionScript`)