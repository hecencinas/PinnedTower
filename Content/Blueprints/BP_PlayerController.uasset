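; Player controller for a tower game where the player drags an arrow on the HUD to aim and fire every tower in the level.
; It creates the in-game HUD with UI-only input and listens to BP_PlayerState updates, enabling drag detection on entering the Aiming state.
; Drag updates turn all cached towers to the drawn angle flipped by 180 degrees.
; Ending a drag fires them all if the player state accepts the shot.
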(event `self.ReceiveBeginPlay`
  (bind _outactors (`GameplayStatics.GetAllActorsOfClass` "/Game/Blueprints/BP_Tower.BP_Tower_C"))
  (set `self.Towers` _outactors)
  (bind _returnvalue (`|CreateWidget` "/Game/Blueprints/WBP_InGameHUD.WBP_InGameHUD_C" self))
  (set `self.InGameHUD` _returnvalue)
  (`UserWidget.AddToViewport` (`self.InGameHUD`) 0)
  (`WidgetBlueprintLibrary.SetInputMode_UIOnlyEx` self (`self.InGameHUD`))
  (set `self.bShowMouseCursor` true)
  (bind _asbp_player_state (cast `/Game/Blueprints/BP_PlayerState` (`GameplayStatics.GetPlayerState` 0)))
  (bind _output_get (set `self.PlayerStateRef` _asbp_player_state))
  (add `/Game/Blueprints/BP_PlayerState.PlayerStateUpdate` _output_get (`|CreateDelegate` :!event `OnPlayerStateUpdate`)))

(event `UpdateToAimState`
  (add `/Game/Blueprints/WBP_InGameHUD.NotifyArrowDrawUpdate` (`self.InGameHUD`) (`|CreateDelegate` :!event `UpdateAngle`))
  (add `/Game/Blueprints/WBP_InGameHUD.NotifyDrawEnded` (`self.InGameHUD`) (`|CreateDelegate` :!event `Shoot`))
  (`/Game/Blueprints/WBP_InGameHUD.EnableArrowDragDetection` (`self.InGameHUD`)))

(event `StopAimState`
  (`/Game/Blueprints/WBP_InGameHUD.DisableArrowDragDetection` (`self.InGameHUD`))
  (clear `/Game/Blueprints/WBP_InGameHUD.NotifyArrowDrawUpdate` (`self.InGameHUD`))
  (clear `/Game/Blueprints/WBP_InGameHUD.NotifyDrawEnded` (`self.InGameHUD`)))

(event `UpdateAngle`
  (bind _cur_angle (`/Game/Blueprints/WBP_InGameHUD.Cur Angle` (`self.InGameHUD`)))
  (for _array_element (`self.Towers`)
    (if (> _cur_angle 0.0)
      (`/Game/Blueprints/BP_Tower.AskToTurn` _array_element (- _cur_angle 180.0))
      (else
        (`/Game/Blueprints/BP_Tower.AskToTurn` _array_element (+ _cur_angle 180.0))))))

(event `Shoot`
  (bind _ok (`/Game/Blueprints/BP_PlayerState.PlayerTriedShot` (`self.PlayerStateRef`)))
  (if _ok
    (`self.StopAimState`)
    (for _array_element (`self.Towers`)
      (`/Game/Blueprints/BP_Tower.Fire` _array_element))))

(event `OnPlayerStateUpdate`
  (bind _currentstate (`/Game/Blueprints/BP_PlayerState.GetCurrentPlayerState` (`self.PlayerStateRef`)))
  (if (`|EnumInequality` _currentstate (`self.LastProcessedState`))
    (bind _output_get (set `self.LastProcessedState` _currentstate))
    (switch `/Game/Blueprints/EPlayerState` _output_get
      (:`NewEnumerator0`
        (`self.UpdateToAimState`)))))

(fn `UserConstructionScript`)