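; BP_NormalProjectile is a bouncing projectile that notifies BP_PlayerState when the last one of its class is destroyed.
; Bounces play random sounds, except against BP_NormalEnemy, and increment a counter.
; At the DestroyOnBounce threshold, it loops over projectiles calling DestroyActor without an explicit target if no enemies remain.
; Below the threshold, it zeroes DestroyOnBounce; the destruction sound is unconnected.
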(event `self.ReceiveBeginPlay`)

(event `self.ReceiveDestroyed`
  (`|ExecutionSequence`
    (:`then_1`
      (bind _outactors (`GameplayStatics.GetAllActorsOfClass` "BP_NormalProjectile_C"))
      (if (== (- (`KismetArrayLibrary.Array_Length` _outactors) 1) 0)
        (bind _asbp_player_state (cast `/Game/Blueprints/BP_PlayerState` (`GameplayStatics.GetPlayerState` 0)))
        (`/Game/Blueprints/BP_PlayerState.NotifyAllProjectilesDestroyed` _asbp_player_state)))))

(event `self.ProjectileMovement.OnProjectileBounce`
  (params (ImpactResult :type "HitResult Structure (by ref)") (ImpactVelocity :type "Vector Structure (by ref)"))
  (`|ExecutionSequence`
    (:`then_0`
      (if (!= ImpactResult_HitActor "/Game/Blueprints/Enemies/BP_NormalEnemy.BP_NormalEnemy")
        (`/Game/Blueprints/BPL_AudioHelper.PlayRandomSound` (`self.SoundsWhenBounce`) ImpactResult_Location)))
    (:`then_1`
      (bind _result (`/Engine/EditorBlueprintResources/StandardMacros.IncrementInt` (`self.CurrentBounceCount`))
        (:`  `
          (if (>= _result (`self.DestroyOnBounce`))
            (bind _outactors (`GameplayStatics.GetAllActorsOfClass` "/Game/Blueprints/Enemies/BP_NormalEnemy.BP_NormalEnemy_C"))
            (if (<= (`KismetArrayLibrary.Array_Length` _outactors) 0)
              (bind _outactors_2 (`GameplayStatics.GetAllActorsOfClass` "BP_NormalProjectile_C"))
              (for _ _outactors_2
                (`self.K2_DestroyActor`)))
            (else
              (set `self.DestroyOnBounce` 0))))))))

(fn `UserConstructionScript`)