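; Utility function library for picking an actor from a weight map using a caller-supplied random factor.
; RandomActorWithWeight2 sorts the map by descending weight, then accumulates weight until it reaches the factor.
; As wired, the loop always reads index 0, so only the heaviest entry's key can be selected.
; A separate helper sums weights; the picker's own total-and-roll nodes are disconnected.
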(fn `CalculateMaxActorRandomWeight2`
  (params (PossibleActorValues :type "Array of Float (double-precision)"))
  (returns (TotalWeight1 :type "Float (double-precision)"))
  (locals (TotalWeight :type "Float (double-precision)" :default 0.0))
  ;[1 1 1] Get total weight
  (for _array_element PossibleActorValues
    (set `local.TotalWeight` (+ (`local.TotalWeight`) _array_element)))
  (return (`local.TotalWeight`)))

(fn `RandomActorWithWeight2`
  (params (PossibleActors :type "Map of Actor Class Reference to Float (double-precision)") (RandomFactor :type "Float (double-precision)"))
  (returns (SelectedActor :type "Actor Class Reference"))
  (locals (TotalWeight :type "Float (double-precision)" :default 0.0) (RandomWeight :type "Float (double-precision)" :default 0.0) (CurWeight :type "Float (double-precision)") (PosibleActorsValues :type "Array of Float (double-precision)") (PossibleActorsKeys :type "Array of Actor Class Reference"))
  (bind _possibleactors1 (`self.SortActorWithWightArray2` null PossibleActors))
  (bind _keys (`BlueprintMapLibrary.Map_Keys` _possibleactors1))
  (set `local.PossibleActorsKeys` _keys)
  (bind _values (`BlueprintMapLibrary.Map_Values` _possibleactors1))
  (set `local.PosibleActorsValues` _values)
  (`|ExecutionSequence`
    (:`then_1`
      (set `local.RandomWeight` RandomFactor))
    (:`then_2`
      ;[1 1 1] Calculate which class to return
      (for _ (range (`KismetArrayLibrary.Array_Length` (`local.PosibleActorsValues`)))
        (bind _output_get (set `local.CurWeight` (+ (`|GetArrayItem` (`local.PosibleActorsValues`)) (`local.CurWeight`))))
        (if (<= (`local.RandomWeight`) _output_get)
          (return (`|GetArrayItem` (`local.PossibleActorsKeys`))))))))

(fn `SortActorWithWightArray2`
  (params (PossibleActors :type "Map of Actor Class Reference to Float (double-precision)"))
  (returns (PossibleActors1 :type "Map of Actor Class Reference to Float (double-precision)"))
  (locals (Ret :type "Map of Actor Class Reference to Float (double-precision)") (InputKeys :type "Array of Actor Class Reference") (InputValues :type "Array of Float (double-precision)"))
  (bind (_indexofmaxvalue _maxvalue) (`KismetMathLibrary.MaxOfFloatArray` (`local.InputValues`)))
  (bind _keys (`BlueprintMapLibrary.Map_Keys` PossibleActors))
  (set `local.InputKeys` _keys)
  (bind _values (`BlueprintMapLibrary.Map_Values` PossibleActors))
  (set `local.InputValues` _values)
  (while (> (`KismetArrayLibrary.Array_Length` (`local.InputValues`)) 0)
    (`BlueprintMapLibrary.Map_Add` (`local.Ret`) (`|GetArrayItem` (`local.InputKeys`) _indexofmaxvalue) _maxvalue)
    (`KismetArrayLibrary.Array_Remove` (`local.InputKeys`) _indexofmaxvalue)
    (`KismetArrayLibrary.Array_Remove` (`local.InputValues`) _indexofmaxvalue))
  (return (`local.Ret`)))