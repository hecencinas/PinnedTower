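; BP_GameStateBase manages the turn flow of a wave-based game, tracking game state, wave count, hit combos and game loss.
; It listens to BP_PlayerState updates, accepting only ordered Aiming, Shooting and Turn Standby transitions; standby resets the combo and switches game state.
; Notify functions take spawn, hit and enemy-finished reports and broadcast through dispatchers, some delayed by timers.
; With no enemies left at standby, it ends the enemy turn itself.
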(event `self.ReceiveBeginPlay`
  (bind _output_get (set `self.PlayerState` (cast `/Game/Blueprints/BP_PlayerState` (`GameplayStatics.GetPlayerState` 0) :!pure true)))
  (add `/Game/Blueprints/BP_PlayerState.PlayerStateUpdate` _output_get (`|CreateDelegate` :!event `OnPlayerStateUpdate`)))

(fn `AllowUpdateProcessedPlayerState`
  (params (NewState :type "/Game/Blueprints/EPlayerState Enum" :default "NewEnumerator3"))
  (returns (OK :type Boolean))
  (bind _lastprocessedplayerstate (`self.LastProcessedPlayerState`))
  (bind _returnvalue (`|EnumEquality` _lastprocessedplayerstate "NewEnumerator3"))
  (switch `/Game/Blueprints/EPlayerState` NewState
    (:`NewEnumerator3`
      (set `self.LastProcessedPlayerState` NewState)
      (return true))
    (:`NewEnumerator0`
      (if (or _returnvalue (`|EnumEquality` _lastprocessedplayerstate "NewEnumerator2"))
        _
        (else
          (return false))))
    (:`NewEnumerator1`
      (if (or _returnvalue (`|EnumEquality` _lastprocessedplayerstate "NewEnumerator0"))
        _
        (else
          (return false))))
    (:`NewEnumerator2`
      (if (or _returnvalue (`|EnumEquality` _lastprocessedplayerstate "NewEnumerator1"))
        _
        (else
          (return false)))))
  (set `self.LastProcessedPlayerState` NewState)
  (return true))

(fn `EndEnemyTurn`
  (`self.NotifiedEnemyActionsEnded`))

(fn `GameStateUpdateDispatch`
  (`self.GameStateUpdate`))

(fn `GetBiggestCombo`
  (returns (BiggestComboCount :type Integer))
  (return (`self.BiggestComboCount`)))

(fn `GetCurComboCount`
  (returns (ComboCount :type Integer))
  (return (`self.ComboCount`)))

(fn `GetCurGameState`
  (returns (GameState :type "/Game/Blueprints/EGameState Enum"))
  (return (`self.GameState`)))

(fn `GetCurWaveCount`
  (returns (WaveCount :type Integer))
  (return (`self.WaveCount`)))

(fn `GetLastWave`
  (returns (WaveCount :type Integer))
  (return (`self.WaveCount`)))

(fn `NotifyEnemiesActionFinished`
  (`KismetSystemLibrary.K2_SetTimer` null "EndEnemyTurn" 1.0))

(fn `NotifyEnemiesSpawned`
  (`/Engine/EditorBlueprintResources/StandardMacros.IncrementInt` (`self.WaveCount`)
    (:`  `
      (set `self.GameState` "NewEnumerator1")
      (`self.GameStateUpdateDispatch`))))

(fn `NotifyEnemyHit`
  (`/Engine/EditorBlueprintResources/StandardMacros.IncrementInt` (`self.ComboCount`)
    (:`  `
      (`self.ComboUpdate`)
      (if (> (`self.ComboCount`) (`self.BiggestComboCount`))
        (set `self.BiggestComboCount` (`self.ComboCount`))))))

(fn `NotifyGameStateUpdate`
  (params (Time :type "Float (single-precision)"))
  (if (> Time 0.0)
    (`KismetSystemLibrary.K2_SetTimer` null "GameStateUpdateDispatch" Time)
    (else
      (`KismetSystemLibrary.K2_SetTimer` null "GameStateUpdateDispatch" 0.1))))

(fn `NotifyPlayerHit`
  (`self.GameLost`))

(fn `OnPlayerStateUpdate`
  (bind _currentstate (`/Game/Blueprints/BP_PlayerState.GetCurrentPlayerState` (`self.PlayerState`)))
  (bind _ok (`self.AllowUpdateProcessedPlayerState` _currentstate))
  (if _ok
    (switch `/Game/Blueprints/EPlayerState` (`self.LastProcessedPlayerState`)
      (:`NewEnumerator2`
        (`|ExecutionSequence`
          (:`then_0`
            (set `self.ComboCount` 0)
            (`self.ComboUpdate`))
          (:`then_1`
            (set `self.GameState` "NewEnumerator2")
            (`self.NotifyGameStateUpdate` 0.0)
            (bind _outactors (`GameplayStatics.GetAllActorsOfClass` "/Game/Blueprints/BP_Enemy.BP_Enemy_C"))
            (if (<= (`KismetArrayLibrary.Array_Length` _outactors) 0)
              (`KismetSystemLibrary.K2_SetTimer` null "NotifyEnemiesActionFinished" 0.1))))))))

(fn `UserConstructionScript`)