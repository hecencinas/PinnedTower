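; Game mode that spawns waves, presumably of enemies, at BP_EnemySpawnPoint actors whenever BP_GameStateBase reports enemy actions ended.
; BeginPlay caches the spawn points, binds to that game state notification and, after a short timer, calls NotifyEnemiesSpawned.
; SpawnNextWave makes a random number of random point picks, skips indices already used, then notifies the game state.
; IndexTaken is never cleared here, so used points stay excluded from later waves.
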(event `self.ReceiveBeginPlay`
  (bind _outactors (`GameplayStatics.GetAllActorsOfClass` "/Game/Blueprints/BP_EnemySpawnPoint.BP_EnemySpawnPoint_C"))
  (set `self.EnemySpawnPoints` _outactors)
  (bind _asbp_game_state_base (cast `/Game/Blueprints/BP_GameStateBase` (`GameplayStatics.GetGameState`)))
  (bind _output_get (set `self.GameStateRef` _asbp_game_state_base))
  (add `/Game/Blueprints/BP_GameStateBase.NotifiedEnemyActionsEnded` _output_get (`|CreateDelegate` :!event `OnEnenmyActionsEnd`))
  (`KismetSystemLibrary.K2_SetTimer` _output_get "NotifyEnemiesSpawned" 0.1))

(fn `OnEnenmyActionsEnd`
  (`self.SpawnNextWave`))

(fn `SpawnNextWave`
  (locals (IndexTaken :type "Set of Integer") (QntySpawns :type Integer :default 0) (TryingToSpawn :type Integer :default 0))
  (bind _returnvalue (`KismetMathLibrary.RandomIntegerInRange` 0 (- (`KismetArrayLibrary.Array_Length` (`self.EnemySpawnPoints`)) 1)))
  (bind _output_get (set `local.QntySpawns` _returnvalue))
  (for _ (range (+ _output_get 1))
    (bind _output_get_2 (set `local.TryingToSpawn` _returnvalue))
    (if (not (`BlueprintSetLibrary.Set_Contains` (`local.IndexTaken`) _output_get_2))
      (`BlueprintSetLibrary.Set_Add` (`local.IndexTaken`) _output_get_2)
      (`|SpawnActorFromClass` "/Game/Blueprints/BP_Enemy.BP_Enemy_C" (`self.GetTransform` (`|GetArrayItem` (`self.EnemySpawnPoints`) _output_get_2)) "Undefined" "OverrideRootScale" null null)))
  (`/Game/Blueprints/BP_GameStateBase.NotifyEnemiesSpawned` (`self.GameStateRef`)))

(fn `UserConstructionScript`)