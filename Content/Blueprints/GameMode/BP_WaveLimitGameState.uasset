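; BP_WaveLimitGameState is a game state for a mode with a capped number of waves.
; NotifyEnemiesSpawned runs the parent logic while WaveCount is below MaxWave, otherwise it switches the GameState enum and broadcasts the update.
; NotifyWining triggers the game-won call, and GetMaxWave exposes the limit.
; GetNextLevelName forwards to BP_WaveLimitMode, the game mode.
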(fn `GetMaxWave`
  (returns (MaxWave :type Integer))
  (return (`self.MaxWave`)))

(fn `GetNextLevelName`
  (returns (NextLevelName :type Name))
  (bind _nextlevelname (`/Game/Blueprints/GameMode/BP_WaveLimitMode.GetNextLevelName` (cast `/Game/Blueprints/GameMode/BP_WaveLimitMode` (`GameplayStatics.GetGameMode`) :!pure true)))
  (return _nextlevelname))

(fn `NotifyEnemiesSpawned`
  (if (< (`self.WaveCount`) (`self.MaxWave`))
    (`parent.NotifyEnemiesSpawned`)
    (else
      (set `self.GameState` "NewEnumerator1")
      (`self.GameStateUpdateDispatch`))))

(fn `NotifyWining`
  (`self.GameWon`))

(fn `UserConstructionScript`
  (`parent.UserConstructionScript`))