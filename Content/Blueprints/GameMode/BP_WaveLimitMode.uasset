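; BP_WaveLimitMode is a wave-based game mode that caps the number of enemy waves and declares a win once the last is cleared.
; Its SpawnNextWave override runs the parent spawn while the current wave count is below the max from BP_WaveLimitGameState.
; At the limit, it counts remaining BP_Enemy actors and notifies the game state of a win if none remain, otherwise that enemies have spawned.
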(event `self.ReceiveBeginPlay`
  (`parent.ReceiveBeginPlay`))

(fn `SpawnNextWave`
  (bind _gamestateref (`self.GameStateRef`))
  (bind _wavecount (`/Game/Blueprints/GameMode/BP_GameStateBase.GetCurWaveCount` _gamestateref))
  (if (< _wavecount (`/Game/Blueprints/GameMode/BP_WaveLimitGameState.GetMaxWave` (cast `/Game/Blueprints/GameMode/BP_WaveLimitGameState` _gamestateref :!pure true)))
    (`parent.SpawnNextWave`)
    (else
      (bind _outactors (`GameplayStatics.GetAllActorsOfClass` "/Game/Blueprints/BP_Enemy.BP_Enemy_C"))
      (if (< (`KismetArrayLibrary.Array_Length` _outactors) 1)
        (`/Game/Blueprints/GameMode/BP_WaveLimitGameState.NotifyWining` (cast `/Game/Blueprints/GameMode/BP_WaveLimitGameState` (`self.GameStateRef`) :!pure true))
        (else
          (`/Game/Blueprints/GameMode/BP_GameStateBase.NotifyEnemiesSpawned` (`self.GameStateRef`)))))))

(fn `UserConstructionScript`
  (`parent.UserConstructionScript`))