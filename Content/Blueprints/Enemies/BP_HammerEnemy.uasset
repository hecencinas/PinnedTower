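; BP_HammerEnemy is an enemy whose Act override charges along its negative forward axis in one jump instead of a single step.
; A long line trace snaps it onto BP_LastLine, or one 100-unit cell short of a blocking BP_NormalEnemy.
; It then flags whether it overlaps the last line and notifies the game state that its action finished.
; An Act starting on the last line reports a player hit and destroys the enemy.
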(fn `Act`
  (bind _returnvalue (`SceneComponent.K2_GetComponentLocation` (`self.Box`)))
  (`/Engine/EditorBlueprintResources/StandardMacros.IncrementInt` (`self.ActionsTaken`)
    (:`  `
      (if (`self.OnLastLine`)
        (`/Game/Blueprints/GameMode/BP_GameStateBase.NotifyPlayerHit` (`self.GameStateRef`))
        (`self.K2_DestroyActor`)
        (else
          (`|ExecutionSequence`
            (:`then_0`
              ;[1 1 1] new override
              (bind (_outhit _returnvalue_2) (`KismetSystemLibrary.LineTraceSingleForObjects` _returnvalue (+ (* (`self.GetActorForwardVector`) -100.0 20.0) _returnvalue) (`|MakeArray` "ObjectTypeQuery2" :!type "EObjectTypeQuery Enum") true (`|MakeArray` self :!type "Actor Object Reference")))
              (if _returnvalue_2
                (bind _asbp_last_line (cast `/Game/Blueprints/BP_LastLine` (`.HitActor` (`GameplayStatics.BreakHitResult` _outhit)))
                  (:`then`
                    (`self.K2_AddActorWorldOffset` (- (`self.K2_GetActorLocation` _asbp_last_line) (`self.K2_GetActorLocation`))))
                  (:`CastFailed`
                    (bind _asbp_normal_enemy (cast `/Game/Blueprints/Enemies/BP_NormalEnemy` (`.HitActor` (`GameplayStatics.BreakHitResult` _outhit))))
                    (`self.K2_AddActorWorldOffset` (- (`self.K2_GetActorLocation` _asbp_normal_enemy) (`self.K2_GetActorLocation`) (* (`self.GetActorForwardVector`) -100.0)))))))
            (:`then_1`
              (if (> (`KismetArrayLibrary.Array_Length` (`PrimitiveComponent.GetOverlappingActors` (`self.Box`) "/Game/Blueprints/BP_LastLine.BP_LastLine_C")) 0)
                (set `self.OnLastLine` true))
              (`/Game/Blueprints/GameMode/BP_GameStateBase.NotifyEnemiesActionFinished` (`self.GameStateRef`)))))))))

(fn `UserConstructionScript`
  (`parent.UserConstructionScript`))