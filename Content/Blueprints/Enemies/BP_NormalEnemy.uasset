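; BP_NormalEnemy is a turn-based enemy whose max health grows with the game state's current wave count.
; Projectile hits or overlaps remove one health, notifying the game state and either updating health listeners or destroying it.
; On each Enemy Turn broadcast from the game state, it steps backward along its forward vector and reports finishing.
; Once it overlaps BP_LastLine, its next action instead reports a player hit and destroys itself.
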(event `self.ReceiveBeginPlay`
  (bind _asbp_game_state_base (cast `/Game/Blueprints/GameMode/BP_GameStateBase` (`GameplayStatics.GetGameState`)))
  (bind _output_get (set `self.GameStateRef` _asbp_game_state_base))
  (add `/Game/Blueprints/GameMode/BP_GameStateBase.GameStateUpdate` _output_get (`|CreateDelegate` :!event `OnGameStateUpdate`))
  (bind _wavecount (`/Game/Blueprints/GameMode/BP_GameStateBase.GetCurWaveCount` (`self.GameStateRef`)))
  (set `self.MaxHealth` (+ _wavecount (`self.MaxHealth`)))
  (set `self.CurHealth` (`self.MaxHealth`))
  (bind _aswbp_enemy_health (cast `/Game/Blueprints/Widgets/WBP_EnemyHealth` (`WidgetComponent.GetUserWidgetObject` (`self.HealthWidgetComponent`))))
  (set `self.HealthWidget` _aswbp_enemy_health)
  (`/Game/Blueprints/Widgets/WBP_EnemyHealth.SetOwnerEnemy` (`self.HealthWidget`) self))

(event `self.Box.OnComponentHit`
  (params (HitComponent :type "PrimitiveComponent Object Reference") (OtherActor :type "Actor Object Reference") (OtherComp :type "PrimitiveComponent Object Reference") (NormalImpulse :type "Vector Structure") (Hit :type "HitResult Structure (by ref)"))
  (cast `/Game/Blueprints/Projectiles/BP_NormalProjectile` OtherActor)
  (`self.DecreaseHealth` :!label _label)
  (`/Game/Blueprints/GameMode/BP_GameStateBase.NotifyEnemyHit` (`self.GameStateRef`)))

(event `self.Box.OnComponentBeginOverlap`
  (params (OverlappedComponent :type "PrimitiveComponent Object Reference") (OtherActor :type "Actor Object Reference") (OtherComp :type "PrimitiveComponent Object Reference") (OtherBodyIndex :type Integer) (bFromSweep :type Boolean) (SweepResult :type "HitResult Structure (by ref)"))
  (cast `/Game/Blueprints/Projectiles/BP_NormalProjectile` OtherActor)
  (goto _label))

(fn `Act`
  (`/Engine/EditorBlueprintResources/StandardMacros.IncrementInt` (`self.ActionsTaken`)
    (:`  `
      (if (`self.OnLastLine`)
        (`/Game/Blueprints/GameMode/BP_GameStateBase.NotifyPlayerHit` (`self.GameStateRef`))
        (`self.K2_DestroyActor`)
        (else
          (`self.K2_AddActorWorldOffset` (* (`self.GetActorForwardVector`) -100.0))
          (if (> (`KismetArrayLibrary.Array_Length` (`PrimitiveComponent.GetOverlappingActors` (`self.Box`) "/Game/Blueprints/BP_LastLine.BP_LastLine_C")) 0)
            (set `self.OnLastLine` true))
          (`/Game/Blueprints/GameMode/BP_GameStateBase.NotifyEnemiesActionFinished` (`self.GameStateRef`)))))))

(fn `DecreaseHealth`
  (bind _result (`/Engine/EditorBlueprintResources/StandardMacros.DecrementInt` (`self.CurHealth`))
    (:`  `
      (if (<= _result 0)
        (`self.K2_DestroyActor`)
        (else
          (`self.NotifyHealthChanged`))))))

(fn `GetCurHealth`
  (returns (CurHealth :type Integer) (MaxHealth :type Integer))
  (return (`self.CurHealth`) (`self.MaxHealth`)))

(fn `OnGameStateUpdate`
  (switch `/Game/Blueprints/Data/EGameState` (`/Game/Blueprints/GameMode/BP_GameStateBase.GameState` (`self.GameStateRef`))
    (:`NewEnumerator2`
      (`self.Act`))))

(fn `UserConstructionScript`)