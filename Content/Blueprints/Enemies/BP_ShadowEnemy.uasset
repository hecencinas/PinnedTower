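; Shadow enemy Blueprint that alternates between a solid state and an intangible shadow state as it acts.
; Act runs the parent behavior, then toggles ShadowTurn, switching the Box collision, the mesh's shadow casting and its material together.
; Shadow mode disables collision and shadow casting, and OnLastLine always forces the solid state.
; The event graph holds only disabled placeholder events.
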(fn `Act`
  (`parent.Act`)
  (if (`self.OnLastLine`)
    (`PrimitiveComponent.SetCollisionEnabled` (`self.Box`) "QueryAndPhysics" :!label _label)
    (set `self.ShadowTurn` false)
    (`PrimitiveComponent.SetCastShadow` (`self.StaticMesh`) true)
    (`PrimitiveComponent.SetMaterial` (`self.StaticMesh`) 0 (`self.DefaultMaterial`))
    (elif (`self.ShadowTurn`)
      (goto _label)
      (else
        (`PrimitiveComponent.SetCollisionEnabled` (`self.Box`) "NoCollision")
        (set `self.ShadowTurn` true)
        (`PrimitiveComponent.SetCastShadow` (`self.StaticMesh`) false)
        (`PrimitiveComponent.SetMaterial` (`self.StaticMesh`) 0 (`self.ShadowModeMaterial`))))))

(fn `UserConstructionScript`
  (`parent.UserConstructionScript`))