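; Tower actor that rotates on request and fires bursts of projectiles from a list that grows with bonuses.
; AskToTurn accepts angles within min/max limits, and Tick eases the cylinder's yaw toward the target.
; Fire spawns each listed projectile class at the arrow through a short self-rescheduling timer, then resets the index.
; Its widget component receives the tower as owner, and adding projectiles broadcasts an update notification.
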(event `self.ReceiveBeginPlay`
  (bind _aswbp_tower_projectiles (cast `/Game/Blueprints/WBP_TowerProjectiles` (`WidgetComponent.GetUserWidgetObject` (`self.ProjectilesQtyWidgetComp`))))
  (`/Game/Blueprints/WBP_TowerProjectiles.SetOwnerTower` _aswbp_tower_projectiles self))

(event `self.ReceiveTick`
  (params (DeltaSeconds :type "Float (single-precision)"))
  (bind (_returnvalue_roll _returnvalue_pitch _returnvalue_yaw) (`KismetMathLibrary.BreakRotator` (`SceneComponent.K2_GetComponentRotation` (`self.TowerCylinder1`))))
  (bind (_returnvalue_roll_2 _returnvalue_pitch_2 _returnvalue_yaw_2) (`KismetMathLibrary.BreakRotator` (`SceneComponent.K2_GetComponentRotation` (`self.TowerCylinder1`))))
  (if (`self.IsTurning`)
    (`SceneComponent.K2_SetWorldRotation` (`self.TowerCylinder1`) (`KismetMathLibrary.MakeRotator` 0.0 0.0 (`KismetMathLibrary.FInterpTo` _returnvalue_yaw (`self.NextAngle`) DeltaSeconds 5.0)) false false)
    (set `self.IsTurning` (!= _returnvalue_yaw_2 (`self.NextAngle`)))))

(event `AskToTurn`
  (params (NextAngle :type "Float (double-precision)"))
  (if (and (`self.CanTurn`) (> NextAngle (`self.MinTurn`)) (< NextAngle (`self.MaxTurn`)) (!= NextAngle (`self.NextAngle`)))
    (set `self.NextAngle` NextAngle)
    (set `self.IsTurning` true)))

(event `Fire`
  (`self.FireLoop`))

(event `NotifyBonus`
  (params (Selection :type "/Game/Blueprints/EBonusType Enum" :default "NewEnumerator0"))
  (switch `/Game/Blueprints/EBonusType` Selection
    (:`NewEnumerator0`
      (`self.AddProjectileToSpawn` "/Game/Blueprints/BP_NormalProjectile.BP_NormalProjectile_C"))))

(fn `AddProjectileToSpawn`
  (params (NewItem :type "/Game/Blueprints/BP_NormalProjectile Class Reference"))
  (`KismetArrayLibrary.Array_Add` (`self.ProjectilesToSpawn`) NewItem)
  (`self.NotifyProjectilesToSpawnUpdated`))

(fn `FireLoop`
  (bind _returnvalue (+ (`self.LastShotIdx`) 1))
  (if (< (`self.LastShotIdx`) (`KismetArrayLibrary.Array_Length` (`self.ProjectilesToSpawn`)))
    (`|SpawnActorFromClass` (`|GetArrayItem` (`self.ProjectilesToSpawn`) (`self.LastShotIdx`)) (`SceneComponent.K2_GetComponentToWorld` (`self.Arrow`)) "Undefined" "OverrideRootScale" self null)
    (if (>= _returnvalue (`KismetArrayLibrary.Array_Length` (`self.ProjectilesToSpawn`)))
      (set `self.LastShotIdx` 0)
      (else
        (set `self.LastShotIdx` _returnvalue)
        (`KismetSystemLibrary.K2_SetTimer` null "FireLoop" 0.1)))))

(fn `GetProjectilesQty`
  (returns (ReturnValue :type Integer))
  (return (`KismetArrayLibrary.Array_Length` (`self.ProjectilesToSpawn`))))

(fn `UserConstructionScript`)