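; Player state for a turn-based shooting game, tracking the player's progress through a turn as a three-step state machine.
; It listens to BP_GameStateBase updates and resets to the first state when Player Turn begins.
; PlayerTriedShot accepts a shot only from that state and advances it, then NotifyAllProjectilesDestroyed moves it to the final state.
; Each change broadcasts PlayerStateUpdate through a short timer rather than immediately.
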(event `self.ReceiveBeginPlay`
  (bind _asbp_game_state_base (cast `/Game/Blueprints/GameMode/BP_GameStateBase` (`GameplayStatics.GetGameState`)))
  (bind _output_get (set `self.GameStateRef` _asbp_game_state_base))
  (add `/Game/Blueprints/GameMode/BP_GameStateBase.GameStateUpdate` _output_get (`|CreateDelegate` :!event `OnGameStateUpdate`)))

(fn `GetCurrentPlayerState`
  (returns (CurrentState :type "/Game/Blueprints/EPlayerState Enum"))
  (return (`self.CurrentPlayerState`)))

(fn `NotifyAllProjectilesDestroyed`
  (if (and (`|EnumEquality` (`self.CurrentPlayerState`) "NewEnumerator1") (`|EnumEquality` (`self.LastGameState`) "NewEnumerator1"))
    (set `self.CurrentPlayerState` "NewEnumerator2")
    (`self.NotifyNewState` 0.0)))

(fn `NotifyNewState`
  (params (Time :type "Float (single-precision)"))
  (if (> Time 0.0)
    (`KismetSystemLibrary.K2_SetTimer` null "NotifyPlayerStateUpdateDispatch" Time)
    (else
      (`KismetSystemLibrary.K2_SetTimer` null "NotifyPlayerStateUpdateDispatch" 0.1))))

(fn `NotifyPlayerStateUpdateDispatch`
  (`self.PlayerStateUpdate`))

(fn `OnGameStateUpdate`
  (bind _gamestate (`/Game/Blueprints/GameMode/BP_GameStateBase.GetCurGameState` (`self.GameStateRef`)))
  (if (`|EnumInequality` _gamestate (`self.LastGameState`))
    (bind _output_get (set `self.LastGameState` _gamestate))
    (switch `/Game/Blueprints/EGameState` _output_get
      (:`NewEnumerator1`
        (set `self.CurrentPlayerState` "NewEnumerator0")
        (`self.NotifyNewState` 0.1)))))

(fn `PlayerTriedShot`
  (returns (OK :type Boolean))
  (bind _gamestate (`/Game/Blueprints/GameMode/BP_GameStateBase.GetCurGameState` (`self.GameStateRef`)))
  (if (and (`|EnumEquality` (`self.LastGameState`) _gamestate) (`|EnumEquality` _gamestate "NewEnumerator1") (`|EnumEquality` (`self.CurrentPlayerState`) "NewEnumerator0"))
    (set `self.CurrentPlayerState` "NewEnumerator1")
    (`self.NotifyNewState` 0.0)
    (return true)
    (else
      (return false))))

(fn `UserConstructionScript`)